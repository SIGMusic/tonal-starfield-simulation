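; Star actor that drifts along a set direction and removes itself once it travels too far along negative Y.
; Each tick it sets the actor location to the StarMesh relative location plus the normalized Direction times Speed, without sweep or delta-time scaling.
; It destroys itself when the mesh's relative Y drops below a fixed threshold.
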(event `self.ReceiveTick`
  (params (DeltaSeconds :type "Float (single-precision)"))
  ;[1 1 1] onTick (move star and check for removal)
  (`self.K2_SetActorLocation` (+ (`SceneComponent.RelativeLocation` (`self.StarMesh`)) (* (`KismetMathLibrary.Normal` (`self.Direction`)) (`self.Speed`))))
  (if (> -3000.0 (.y (`SceneComponent.RelativeLocation` (`self.StarMesh`))))
    (`self.K2_DestroyActor`)))

(fn `UserConstructionScript`)