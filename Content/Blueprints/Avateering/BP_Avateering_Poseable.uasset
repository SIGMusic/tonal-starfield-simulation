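; Blueprint actor for Kinect avateering that drives a poseable mesh from a tracked player body.
; On BeginPlay it caches the Kinect player controller and applies the Smoothing setting to its KinectPoseableMesh component.
; Each tick it reads the centered body from the controller and sets it as the mesh's target body.
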(event `self.ReceiveBeginPlay`
  (bind _askinectplayercontroller (cast `KinectPlayerController` (`GameplayStatics.GetPlayerController` 0)))
  (set `self.KPC` _askinectplayercontroller)
  (set `KinectPoseableMeshComponent.IsSmoothing` (`self.Smoothing`) (`self.KinectPoseableMesh`)))

(event `self.ReceiveTick`
  (params (DeltaSeconds :type "Float (single-precision)"))
  (bind _centeredbody (`KinectPlayerController.GetCenteredBody` (`self.KPC`)))
  (set `KinectPoseableMeshComponent.TargetBody` _centeredbody (`self.KinectPoseableMesh`)))

(fn `UserConstructionScript`)