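; BP_TestActor is a test actor that shows the Kinect-tracked hands of the centered body as two meshes.
; On BeginPlay it casts player controller 0 to KinectPlayerController and stores it.
; Each tick it asks that controller for the centered body and its absolute left and right hand joint positions, then sets those directly as the relative locations of LeftHandMesh and RightHandMesh.
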(event `self.ReceiveBeginPlay`
  ;[1 1 1] OnBeginPlay
  (bind _askinectplayercontroller (cast `KinectPlayerController` (`GameplayStatics.GetPlayerController` 0)))
  (set `self.myKinectPlayerController` _askinectplayercontroller))

(event `self.ReceiveTick`
  (params (DeltaSeconds :type "Float (single-precision)"))
  (bind _centeredbody (`KinectPlayerController.GetCenteredBody` (`self.myKinectPlayerController`)))
  (bind _returnvalue (`KinectPlayerController.GetJointAbsolutePosition` (`self.myKinectPlayerController`) "HandLeft" _centeredbody))
  (`SceneComponent.SetRelativeLocation` (`self.LeftHandMesh`) _returnvalue false)
  (bind _returnvalue_2 (`KinectPlayerController.GetJointAbsolutePosition` (`self.myKinectPlayerController`) "HandRight" _centeredbody))
  (`SceneComponent.SetRelativeLocation` (`self.RightHandMesh`) _returnvalue_2 false))

(fn `UserConstructionScript`)